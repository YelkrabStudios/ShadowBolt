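; Parkour turn post that swings the player along a short spline when jump is held inside its trigger, labelled as pipe slide logic.
; Overlap starts a looping timer that polls jump input, then fires once per overlap if a forward trace is clear.
; Chained MoveComponentTo calls carry the capsule through the spline points while a timeline steers view toward Cube3, adding shake, speed and FOV changes.
; The construction script snaps Cube3 to the third spline point.
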(event `self.DetectCollision.OnComponentBeginOverlap`
  (params (OverlappedComponent :type "PrimitiveComponent Object Reference") (OtherActor :type "Actor Object Reference") (OtherComp :type "PrimitiveComponent Object Reference") (OtherBodyIndex :type Integer) (bFromSweep :type Boolean) (SweepResult :type "HitResult Structure (by ref)"))
  ;[1 0 0.0652] Pipe Slide Logic
  (if (== OtherActor (`/Game/Characters/Player/FunctionLibrary/BP_PlayerFunctionLibrary.Get Player Character`))
    (set `self.InOverlap` true)
    (bind _returnvalue (`KismetSystemLibrary.K2_SetTimerDelegate` (delegate `PipeSldeCheck`) 0.1 true))
    (set `self.CheckTimer` _returnvalue)))

(event `PipeSldeCheck`
  (bind _returnvalue (`SplineComponent.GetLocationAtSplinePoint` (`self.Spline`) 0 "World"))
  ;[1 0 0.0652] Pipe Slide Logic
  (if (and (`/Game/Characters/Player/Blueprints/BP_PlayerCharacter.varJumpKeyDown` (`/Game/Characters/Player/FunctionLibrary/BP_PlayerFunctionLibrary.Get Player Character`)) (`self.InOverlap`))
    (`/Engine/EditorBlueprintResources/StandardMacros.DoOnce` false :!label _label
      (:`Completed`
        (bind (_outhit _returnvalue_2) (`KismetSystemLibrary.LineTraceSingle` :`Start` _returnvalue :`End` (+ _returnvalue (* (`SceneComponent.GetForwardVector` (`/Game/Characters/Player/FunctionLibrary/BP_PlayerFunctionLibrary.GetCapsuleComp`)) 100.0)) :`TraceChannel` "TraceTypeQuery2" :`DrawDebugType` "Persistent" :`bIgnoreSelf` false :`DrawTime` 0.0))
        (if (not _returnvalue_2)
          (set `/Game/Characters/Player/Blueprints/BP_PlayerCharacter.varMovementState` "NewEnumerator13" (`/Game/Characters/Player/FunctionLibrary/BP_PlayerFunctionLibrary.Get Player Character`))
          (`|ExecutionSequence`
            (:`then_0`
              (`Timeline|Timeline_0` :!via `PlayFromStart`
                (:`Update`
                  (`Controller.SetControlRotation` (`GameplayStatics.GetPlayerController` 0) (`KismetMathLibrary.RInterpTo` (`Pawn.GetControlRotation` (`/Game/Characters/Player/FunctionLibrary/BP_PlayerFunctionLibrary.Get Player Character`)) (`KismetMathLibrary.FindLookAtRotation` (`self.K2_GetActorLocation` (`/Game/Characters/Player/FunctionLibrary/BP_PlayerFunctionLibrary.Get Player Character`)) (`SceneComponent.K2_GetComponentLocation` (`self.Cube3`))) (`GameplayStatics.GetWorldDeltaSeconds`) 8.0))
                  (`/Game/Characters/Player/FunctionLibrary/BP_PlayerFunctionLibrary.PlayCameraShake` "/Game/Characters/Player/Misc/CameraShake/Parkour/Pipe/BP_RightPipeCameraShake.BP_RightPipeCameraShake_C" 1.5)
                  (`/Game/Characters/Player/FunctionLibrary/BP_PlayerFunctionLibrary.PlayerSpeed` "NewEnumerator1" 2.0)
                  (`/Game/Characters/Player/FunctionLibrary/BP_PlayerFunctionLibrary.UpdateFOV` 90.0 3.0))))
            (:`then_1`
              (`KismetSystemLibrary.MoveComponentTo` (`/Game/Characters/Player/FunctionLibrary/BP_PlayerFunctionLibrary.GetCapsuleComp`) (`SplineComponent.GetLocationAtSplinePoint` (`self.Spline`) 1 "World") (struct) false true)
              (`KismetSystemLibrary.MoveComponentTo` (`/Game/Characters/Player/FunctionLibrary/BP_PlayerFunctionLibrary.GetCapsuleComp`) (`SplineComponent.GetLocationAtSplinePoint` (`self.Spline`) 2 "World") (struct) false true)
              (set `/Game/Characters/Player/Blueprints/BP_PlayerCharacter.varMovementState` "NewEnumerator1" (`/Game/Characters/Player/FunctionLibrary/BP_PlayerFunctionLibrary.Get Player Character`))
              (`KismetSystemLibrary.Delay` 0.2)
              (`/Game/Characters/Player/FunctionLibrary/BP_PlayerFunctionLibrary.PlayCameraShake` "/Game/Characters/Player/Misc/CameraShake/Movement/Jump/BP_JumpeEndCameraShake.BP_JumpeEndCameraShake_C" 2.0))))))))

(event `self.DetectCollision.OnComponentEndOverlap`
  (params (OverlappedComponent :type "PrimitiveComponent Object Reference") (OtherActor :type "Actor Object Reference") (OtherComp :type "PrimitiveComponent Object Reference") (OtherBodyIndex :type Integer))
  (bind _player_character (`/Game/Characters/Player/FunctionLibrary/BP_PlayerFunctionLibrary.Get Player Character`))
  ;[1 0 0.0652] Pipe Slide Logic
  (if (== OtherActor _player_character)
    (`|ExecutionSequence`
      (:`then_0`
        (set `self.InOverlap` false)
        (set `/Game/Characters/Player/Blueprints/BP_PlayerCharacter.varMovementState` "NewEnumerator4" _player_character))
      (:`then_1`
        (goto _label :!via `Reset`))
      (:`then_2`
        (`KismetSystemLibrary.K2_ClearAndInvalidateTimerHandle` (`self.CheckTimer`))))))

(fn `JumpCheck`)

(fn `UserConstructionScript`
  (bind _cube3 (`self.Cube3`))
  (bind _spline (`self.Spline`))
  (`SceneComponent.K2_SetWorldLocation` _cube3 (`SplineComponent.GetLocationAtSplinePoint` _spline 2 "World") false false)
  (`SceneComponent.K2_SetWorldRotation` _cube3 (`SplineComponent.GetRotationAtSplinePoint` _spline 2 "World") false false))