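; Blueprint function library of shared helpers for the first-person BP_PlayerCharacter, resolved from player index 0.
; Getters expose components, movement state, velocity and control-yaw vectors, while setters handle input locks, health, water state and yaw clamping.
; Speed, FOV and radial blur ease via per-call FInterpTo, and a capsule trace decides whether uncrouching is allowed.
; Point detector, begin-screen widget and notification functions are unfinished stubs.
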(fn `ActiveClimbPoint`
  (returns (Index :type Integer))
  ;[0 0.5 0.04509] Find Active Climb Point
  (return (`/Game/Characters/Player/BPs/BP_PlayerCharacter.varPointDetectorIndex` (`self.Get Player Character` null))))

(fn `AddHealthToPlayer`
  (params (Range :type "Float (double-precision)"))
  (bind _player_character (`self.Get Player Character` null))
  ;[0.07812 0.2593 1] Player Camera Shake
  (set `/Game/Characters/Player/BPs/BP_PlayerCharacter.varHealthCurrent` (`KismetMathLibrary.FClamp` (+ Range (`/Game/Characters/Player/BPs/BP_PlayerCharacter.varHealthCurrent` _player_character)) 0.0 (`/Game/Characters/Player/BPs/BP_PlayerCharacter.varHealthDefault` _player_character)) _player_character))

(fn `ClampYaw`
  (bind _returnvalue (`GameplayStatics.GetPlayerCameraManager` null))
  (bind (_returnvalue_roll _returnvalue_pitch _returnvalue_yaw) (`KismetMathLibrary.BreakRotator` (`SceneComponent.K2_GetComponentRotation` (`self.GetCapsuleComp` null))))
  ;[0.07812 0.2593 1] Clamp Yaw
  (set `PlayerCameraManager.ViewYawMin` (- _returnvalue_yaw 145.0) _returnvalue)
  (set `PlayerCameraManager.ViewYawMax` (+ _returnvalue_yaw 145.0) _returnvalue))

(fn `CrouchCollision`
  (bind _player_character (`self.Get Player Character` null))
  (bind _capsulecomponent (`self.GetCapsuleComp` null))
  (bind _returnvalue (+ (`SceneComponent.K2_GetComponentLocation` _capsulecomponent) (* (`SceneComponent.GetUpVector` _capsulecomponent) 70.0)))
  ;[0.07812 0.2593 1] Crouch Collision
  (`|ExecutionSequence`
    (:`then_0`
      (if (or (`self.IsInState` "NewEnumerator3") (`self.IsInState` "NewEnumerator6") (`self.IsInState` "NewEnumerator1") (`self.IsInState` "NewEnumerator4"))
        (bind (_outhit _returnvalue_2) (`KismetSystemLibrary.CapsuleTraceSingle` :`Start` _returnvalue :`End` _returnvalue :`Radius` 10.0 :`HalfHeight` 30.0 :`TraceChannel` "TraceTypeQuery1" :`bIgnoreSelf` false))
        (if _returnvalue_2
          (set `/Game/Characters/Player/BPs/BP_PlayerCharacter.VarCanUnCrouch` false _player_character)
          (else
            (set `/Game/Characters/Player/BPs/BP_PlayerCharacter.VarCanUnCrouch` true _player_character)))))))

(fn `DisablePlayerInputNotCameraInput`
  (bind _player_character (`self.Get Player Character` null))
  ;[0.07812 0.2593 1] Disable Movement
  (set `/Game/Characters/Player/BPs/BP_PlayerCharacter.VarMovementInput` "NewEnumerator0" _player_character)
  (set `/Game/Characters/Player/BPs/BP_PlayerCharacter.varMouseInput` "NewEnumerator1" _player_character))

(fn `DisablePlayerMovement`
  (bind _player_character (`self.Get Player Character` null))
  ;[0.07812 0.2593 1] Disable Movement
  (set `/Game/Characters/Player/BPs/BP_PlayerCharacter.varMouseInput` "NewEnumerator0" _player_character)
  (set `/Game/Characters/Player/BPs/BP_PlayerCharacter.VarMovementInput` "NewEnumerator0" _player_character))

(fn `EnablePlayerInputNotCameraInput`
  ;[0.07812 0.2593 1] Disable Movement
  (set `/Game/Characters/Player/BPs/BP_PlayerCharacter.VarMovementInput` "NewEnumerator1" (`self.Get Player Character` null)))

(fn `EnablePlayerMovement`
  (bind _player_character (`self.Get Player Character` null))
  ;[0.07812 0.2593 1] Enable Movement
  (`SceneComponent.K2_SetRelativeRotation` (`self.GetCapsuleComp` null) (`/Game/Characters/Player/BPs/BP_PlayerCharacter.varCapsuleBeginRotation` _player_character) false false)
  (set `/Game/Characters/Player/BPs/BP_PlayerCharacter.varMouseInput` "NewEnumerator1" _player_character)
  (set `/Game/Characters/Player/BPs/BP_PlayerCharacter.VarMovementInput` "NewEnumerator1" _player_character)
  (set `/Game/Characters/Player/BPs/BP_PlayerCharacter.varMovementState` "NewEnumerator1" _player_character))

(fn `FrameDetector`
  (returns (`30 FPS` :type Boolean) (`60 FPS` :type Boolean) (`120 FPS` :type Boolean))
  (bind _vardeltaseconds (`/Game/Characters/Player/BPs/BP_PlayerCharacter.varDeltaSeconds` (`self.Get Player Character` null)))
  ;[0 0.5 0.04509] Frame Detector
  (return (or (and (< _vardeltaseconds 0.04) (> _vardeltaseconds 0.02)) (> 0.0 0.02)) (and (< _vardeltaseconds 0.02) (> _vardeltaseconds 0.009)) (and (< _vardeltaseconds 0.009) (> _vardeltaseconds 0.008))))

(fn `Get Player Character`
  (returns (`Player Character` :type "/Game/Characters/Player/BPs/BP_PlayerCharacter Object Reference"))
  ;[0 0.5 0.04509] Get Player Character
  (return (cast `/Game/Characters/Player/BPs/BP_PlayerCharacter` (`GameplayStatics.GetPlayerPawn` null) :!pure true)))

(fn `GetBeginScreenWidget`
  ;[0 0.5 0.04509] Get Player Begin Screen Widget
  (`KismetSystemLibrary.PrintString` null "GETBEGINSCREENWIDGET function not complete")
  (return))

(fn `GetCapsuleComp`
  (returns (CapsuleComponent :type "CapsuleComponent Object Reference"))
  ;[0 0.5 0.04509] Get Player Capsule Component
  (return (`Character.CapsuleComponent` (cast `/Game/Characters/Player/BPs/BP_PlayerCharacter` (`GameplayStatics.GetPlayerPawn` null) :!pure true))))

(fn `GetCharacterForwardVector`
  (returns (`Forward Vector` :type "Vector Structure"))
  ;[0 0.5 0.04509] Get Player Right Vector
  (return (`KismetMathLibrary.GetForwardVector` (`KismetMathLibrary.MakeRotator` 0.0 0.0 (.yaw (`Pawn.GetControlRotation` (`self.Get Player Character` null)))))))

(fn `GetCharacterMovementComp`
  (returns (CharacterMovement :type "CharacterMovementComponent Object Reference"))
  ;[0 0.5 0.04509] Get Player Character Movement Component
  (return (`Character.CharacterMovement` (cast `/Game/Characters/Player/BPs/BP_PlayerCharacter` (`GameplayStatics.GetPlayerPawn` null) :!pure true))))

(fn `GetCharacterRightVector`
  (returns (`Right Vector` :type "Vector Structure"))
  ;[0 0.5 0.04509] Get Player Right Vector
  (return (`KismetMathLibrary.GetRightVector` (`KismetMathLibrary.MakeRotator` 0.0 0.0 (.yaw (`Pawn.GetControlRotation` (`self.Get Player Character` null)))))))

(fn `GetCharacterVectorLength`
  (returns (`Vector Length` :type "Float (double-precision)"))
  ;[0 0.5 0.04509] Get Player Vector Length
  (return (`KismetMathLibrary.VSize` (`Actor.GetVelocity` (`self.Get Player Character` null)))))

(fn `GetFPCameraComp`
  (returns (FirstPersonCamera :type "CameraComponent Object Reference"))
  ;[0 0.5 0.04509] Get Player First Person Camera Component
  (return (`/Game/Characters/Player/BPs/BP_PlayerCharacter.FirstPersonCamera` (cast `/Game/Characters/Player/BPs/BP_PlayerCharacter` (`GameplayStatics.GetPlayerPawn` null) :!pure true))))

(fn `GetMovementState`
  (returns (`Active Player State` :type "/Game/Characters/Player/Enums/Enum_Player_MovementStates Enum"))
  ;[0 0.5 0.04509] Get Player Movement State
  (return (`/Game/Characters/Player/BPs/BP_PlayerCharacter.varMovementState` (cast `/Game/Characters/Player/BPs/BP_PlayerCharacter` (`GameplayStatics.GetPlayerPawn` null) :!pure true))))

(fn `GetPointDetector`
  (returns (`Point Detector` :type "Actor Object Reference"))
  ;[0 0.5 0.04509] Get Player Point Detector
  (`KismetSystemLibrary.PrintString` null "GETPOINTDETECTOR function not complete"))

(fn `InWater`
  (params (InWater :type Boolean))
  ;[0.07812 0.2593 1] In Water Setter
  (set `/Game/Characters/Player/BPs/BP_PlayerCharacter.varIsInWater` InWater (`self.Get Player Character` null)))

(fn `Is Falling`
  (returns (ReturnValue :type Boolean))
  (bind (_returnvalue_x _returnvalue_y _returnvalue_z) (`KismetMathLibrary.BreakVector` (`Actor.GetVelocity` (`self.Get Player Character` null))))
  ;[0 0.5 0.04509] Comment
  (return (<= _returnvalue_z -10.0)))

(fn `IsInAir`
  (returns (ReturnValue :type Boolean))
  ;[0 0.5 0.04509] Is Player In Air?
  (return (`NavMovementComponent.IsFalling` (`self.GetCharacterMovementComp` null))))

(fn `IsInState`
  (params (`Player Movement State` :type "/Game/Characters/Player/Enums/Enum_Player_MovementStates Enum" :default "NewEnumerator0"))
  (returns (ReturnValue :type Boolean))
  ;[0 0.5 0.04509] Is Player In State?
  (return (== `Player Movement State` (`/Game/Characters/Player/BPs/BP_PlayerCharacter.varMovementState` (`self.Get Player Character` null)))))

(fn `IsInWater`
  (returns (`Return Value` :type Boolean))
  ;[0 0.5 0.04509] In Water Setter
  (return (`/Game/Characters/Player/BPs/BP_PlayerCharacter.varIsInWater` (`self.Get Player Character` null))))

(fn `NotificationNOTDONE`
  (params (Notification :type Text))
  ;[0.07812 0.2593 1] Player Camera Shake
  (`KismetSystemLibrary.PrintString` null "NOTIFICATION function not complete"))

(fn `PlayCameraShake`
  (params (Shake :type "CameraShake Class Reference") (Scale :type "Float (double-precision)"))
  ;[0.07812 0.2593 1] Player Camera Shake
  (`PlayerController.ClientStartCameraShake` :`self` (`GameplayStatics.GetPlayerController` null) :`Shake` Shake :`Scale` Scale))

(fn `PlayerSpeed`
  (params (`Player Speed` :type "/Game/Characters/Player/Enums/Enum_PlayerSpeed Enum" :default "NewEnumerator0") (`Switch Speed` :type "Float (double-precision)"))
  (bind _player_character (`self.Get Player Character` null))
  (bind _charactermovement (`self.GetCharacterMovementComp` null))
  (bind _returnvalue (`GameplayStatics.GetWorldDeltaSeconds` null))
  (bind _maxwalkspeed (`CharacterMovementComponent.MaxWalkSpeed` _charactermovement))
  ;[0.07812 0.2593 1] Set Player Speed Smoothly
  (switch `/Game/Characters/Player/Enums/Enum_PlayerSpeed` `Player Speed`
    (:`NewEnumerator0`
      (set `CharacterMovementComponent.MaxWalkSpeed` (`KismetMathLibrary.FInterpTo` _maxwalkspeed (`/Game/Characters/Player/BPs/BP_PlayerCharacter.varMovementSpeed` _player_character) _returnvalue `Switch Speed`) _charactermovement))
    (:`NewEnumerator1`
      (set `CharacterMovementComponent.MaxWalkSpeed` (`KismetMathLibrary.FInterpTo` _maxwalkspeed (`/Game/Characters/Player/BPs/BP_PlayerCharacter.varSprintSpeedMinimum` _player_character) _returnvalue `Switch Speed`) _charactermovement))
    (:`NewEnumerator2`
      (set `CharacterMovementComponent.MaxWalkSpeed` (`KismetMathLibrary.FInterpTo` _maxwalkspeed (`/Game/Characters/Player/BPs/BP_PlayerCharacter.varCrouchSpeed` _player_character) _returnvalue `Switch Speed`) _charactermovement))
    (:`NewEnumerator3`
      (set `CharacterMovementComponent.MaxWalkSpeed` (`KismetMathLibrary.FInterpTo` _maxwalkspeed (`/Game/Characters/Player/BPs/BP_PlayerCharacter.varSlideSpeed` _player_character) _returnvalue `Switch Speed`) _charactermovement))
    (:`NewEnumerator5`
      (set `CharacterMovementComponent.MaxWalkSpeed` (`KismetMathLibrary.FInterpTo` _maxwalkspeed (`/Game/Characters/Player/BPs/BP_PlayerCharacter.VarDodgeSpeed` _player_character) _returnvalue `Switch Speed`) _charactermovement))
    (:`NewEnumerator6`
      (set `CharacterMovementComponent.MaxWalkSpeed` (`KismetMathLibrary.FInterpTo` _maxwalkspeed (`/Game/Characters/Player/BPs/BP_PlayerCharacter.varWallRunningSpeed` _player_character) _returnvalue `Switch Speed`) _charactermovement))))

(fn `RadialBlur`
  (params (Scale :type "Float (double-precision)") (Speed :type "Float (double-precision)"))
  ;[0.07812 0.2593 1] Smooth Radial Blur
  (bind _returnvalue (`KismetMaterialLibrary.GetScalarParameterValue` null "/Game/Material/Scan/MPC_NMCollection.MPC_NMCollection" "BlurBlend"))
  (`KismetMaterialLibrary.SetScalarParameterValue` null "/Game/Material/Scan/MPC_NMCollection.MPC_NMCollection" "BlurBlend" (`KismetMathLibrary.FInterpTo` _returnvalue Scale (`GameplayStatics.GetWorldDeltaSeconds` null) Speed)))

(fn `ResetClampYaw`
  (bind _returnvalue (`GameplayStatics.GetPlayerCameraManager` null))
  ;[0.07812 0.2593 1] Reset Clamp Yaw
  (set `PlayerCameraManager.ViewYawMin` 0.0 _returnvalue)
  (set `PlayerCameraManager.ViewYawMax` 359.998993 _returnvalue))

(fn `UpdateFOV`
  (params (Scale :type "Float (double-precision)") (Speed :type "Float (double-precision)"))
  (bind _firstpersoncamera (`/Game/Characters/Player/BPs/BP_PlayerCharacter.FirstPersonCamera` (`self.Get Player Character` null)))
  ;[0.07812 0.2593 1] Update Camera FOV
  (`CameraComponent.SetFieldOfView` _firstpersoncamera (`KismetMathLibrary.FInterpTo` (`CameraComponent.FieldOfView` _firstpersoncamera) Scale (`GameplayStatics.GetWorldDeltaSeconds` null) Speed)))