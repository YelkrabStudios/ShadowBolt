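; Zipline interactable that the player grabs with jump input inside its trigger and rides from spline start to end.
; On grab, the capsule moves to the start and attaches to AttachPoint while Origin moves linearly at state-based slow or fast timing, with camera shakes and FOV changes.
; Jump or crouch exits early.
; Construction script aligns meshes and cable, flagging splines with over two points or insufficient downward drop.
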(event `self.ReceiveBeginPlay`
  (`self.GetSplinePoints`))

(event `self.Interact.OnComponentBeginOverlap`
  (params (OverlappedComponent :type "PrimitiveComponent Object Reference") (OtherActor :type "Actor Object Reference") (OtherComp :type "PrimitiveComponent Object Reference") (OtherBodyIndex :type Integer) (bFromSweep :type Boolean) (SweepResult :type "HitResult Structure (by ref)"))
  ;[1 0 0.0652] Activate Zipline
  (if (== OtherActor (`/Game/Characters/Player/FunctionLib/BP_PlayerFunctionLibrary.Get Player Character`))
    (`self.EnableInput` (`GameplayStatics.GetPlayerController` 0))
    (`|ExecutionSequence`
      (:`then_0`
        (goto _label :!via `Open`))
      (:`then_1`
        (if (> (`/Game/Characters/Player/BPs/BP_PlayerCharacter.varJumpAxis` (`/Game/Characters/Player/FunctionLib/BP_PlayerFunctionLibrary.Get Player Character`)) 0.0)
          (`/Engine/EditorBlueprintResources/StandardMacros.Gate` true :!label _label
            (:`Exit`
              (`/Engine/EditorBlueprintResources/StandardMacros.DoOnce` false :!label _label_2
                (:`Completed`
                  (`self.Request: Start Zipline`)
                  (set `/Game/Characters/Player/BPs/BP_PlayerCharacter.varMovementState` "NewEnumerator18" (`/Game/Characters/Player/FunctionLib/BP_PlayerFunctionLibrary.Get Player Character`))
                  (`/Game/Characters/Player/FunctionLib/BP_PlayerFunctionLibrary.ClampYaw`)
                  (goto _label :!via `Close`))))))))))

(event `self.Interact.OnComponentEndOverlap`
  (params (OverlappedComponent :type "PrimitiveComponent Object Reference") (OtherActor :type "Actor Object Reference") (OtherComp :type "PrimitiveComponent Object Reference") (OtherBodyIndex :type Integer))
  ;[1 0 0.0652] Activate Zipline
  (if (== OtherActor (`/Game/Characters/Player/FunctionLib/BP_PlayerFunctionLibrary.Get Player Character`))
    (if (`/Game/Characters/Player/FunctionLib/BP_PlayerFunctionLibrary.IsInState` "NewEnumerator18")
      (goto _label_2 :!via `Reset`)
      (else
        (`self.DisableInput` (`GameplayStatics.GetPlayerController` 0))))))

(event `Request: Start Zipline`
  (bind _charactermovement (`/Game/Characters/Player/FunctionLib/BP_PlayerFunctionLibrary.GetCharacterMovementComp`))
  (bind _capsulecomponent (`/Game/Characters/Player/FunctionLib/BP_PlayerFunctionLibrary.GetCapsuleComp`))
  (bind _player_character (`/Game/Characters/Player/FunctionLib/BP_PlayerFunctionLibrary.Get Player Character`))
  (`/Game/Characters/Player/FunctionLib/BP_PlayerFunctionLibrary.PlayCameraShake` "/Game/Characters/Player/Misc/CameraShake/ZipLine/BP_ZipLineStartCameraShake.BP_ZipLineStartCameraShake_C" 1.0)
  (`/Game/Characters/Player/FunctionLib/BP_PlayerFunctionLibrary.DisablePlayerInputNotCameraInput`)
  (if (`/Game/Characters/Player/FunctionLib/BP_PlayerFunctionLibrary.IsInState` "NewEnumerator1")
    (set `self.ZipLineTime` (`self.ZipLineTimeSlow`))
    (else
      (set `self.ZipLineTime` (`self.ZipLineTimeFast`))))
  (set `CharacterMovementComponent.GravityScale` 0.0 _charactermovement)
  (set `MovementComponent.Velocity` (0.0 0.0 0.0) _charactermovement)
  (`KismetSystemLibrary.MoveComponentTo` _capsulecomponent (+ (* (`SceneComponent.GetUpVector` _capsulecomponent) -90.0) (`SplineComponent.GetLocationAtSplinePoint` (`self.ZipLine`) 0 "World")) (`SceneComponent.RelativeRotation` _capsulecomponent) false true 0.3 :!label _label_3)
  (`|ExecutionSequence`
    (:`then_0`
      (`self.K2_AttachToComponent` (`/Game/Characters/Player/FunctionLib/BP_PlayerFunctionLibrary.Get Player Character`) (`self.AttachPoint`) "None" "KeepWorld" "KeepWorld" "SnapToTarget" true)
      (`KismetSystemLibrary.MoveComponentTo` (`self.Origin`) (`self.varEndLocation`) (`SceneComponent.RelativeRotation` (`self.Origin`)) false false (`self.ZipLineTime`) :!label _label_4)
      (`SceneComponent.K2_DetachFromComponent` (`/Game/Characters/Player/FunctionLib/BP_PlayerFunctionLibrary.GetCapsuleComp`) "KeepWorld" "KeepWorld" "KeepWorld" true :!label _label_5)
      (set `CharacterMovementComponent.GravityScale` 1.0 (`/Game/Characters/Player/FunctionLib/BP_PlayerFunctionLibrary.GetCharacterMovementComp`))
      (`/Game/Characters/Player/FunctionLib/BP_PlayerFunctionLibrary.PlayCameraShake` "/Game/Characters/Player/Misc/CameraShake/ZipLine/BP_ZipLineEndCameraShake.BP_ZipLineEndCameraShake_C")
      (`SceneComponent.K2_SetRelativeLocation` (`self.Origin`) (0.0 0.0 0.0) false false)
      (`/Game/Characters/Player/FunctionLib/BP_PlayerFunctionLibrary.EnablePlayerMovement`)
      (if (not (`self.JumpingDropping`))
        (set `/Game/Characters/Player/BPs/BP_PlayerCharacter.varJumpDistance` (`self.CalcJumpDistance`) _player_character)
        (set `/Game/Characters/Player/BPs/BP_PlayerCharacter.varJumpHeight` 0.0 _player_character)
        (`/Game/Characters/Player/BPs/BP_PlayerCharacter.Request: To Jump End` _player_character)
        (`self.DisableInput` (`GameplayStatics.GetPlayerController` 0))
        (`/Game/Characters/Player/FunctionLib/BP_PlayerFunctionLibrary.UpdateFOV` 85.0 1.0)))
    (:`then_1`
      (`TimelineComponent.SetTimelineLength` (`self.RotationTime`) (`self.ZipLineTime`))
      (`Timeline|RotationTime` :!via `PlayFromStart`
        (:`Update`
          (`/Game/Characters/Player/FunctionLib/BP_PlayerFunctionLibrary.PlayCameraShake` "/Game/Characters/Player/Misc/CameraShake/Parkour/Pipe/BP_PipeSlideDownCameraShake1.BP_PipeSlideDownCameraShake1_C" 1.0)
          (`/Game/Characters/Player/FunctionLib/BP_PlayerFunctionLibrary.UpdateFOV` 130.0 0.6))))))

(event `InputAction|JumpEnd`
  (params (Key :type "Key Structure"))
  (bind _player_character (`/Game/Characters/Player/FunctionLib/BP_PlayerFunctionLibrary.Get Player Character`))
  (:`Pressed`
    (if (`/Game/Characters/Player/FunctionLib/BP_PlayerFunctionLibrary.IsInState` "NewEnumerator18")
      (if (> (`KismetMathLibrary.Vector_Distance` (`SceneComponent.K2_GetComponentLocation` (`self.SM_ZipLine`)) (`self.K2_GetActorLocation` (`/Game/Characters/Player/FunctionLib/BP_PlayerFunctionLibrary.Get Player Character`))) 600.0)
        (set `self.JumpingDropping` true)
        (set `/Game/Characters/Player/BPs/BP_PlayerCharacter.varJumpDistance` (`/Game/Characters/Player/BPs/BP_PlayerCharacter.varJumpDistanceZPing` _player_character) _player_character)
        (set `/Game/Characters/Player/BPs/BP_PlayerCharacter.varJumpHeight` 100.0 _player_character)
        (`/Game/Characters/Player/FunctionLib/BP_PlayerFunctionLibrary.PlayCameraShake` "/Game/Characters/Player/Misc/CameraShake/ZipLine/BP_ZipLineJumpUp.BP_ZipLineJumpUp_C" 1.0)
        (`KismetSystemLibrary.Delay` 0.6)
        (`/Game/Characters/Player/FunctionLib/BP_PlayerFunctionLibrary.PlayCameraShake` "/Game/Characters/Player/Misc/CameraShake/ZipLine/BP_ZipLineJumpDown.BP_ZipLineJumpDown_C" 1.0)
        (`KismetSystemLibrary.Delay` 0.2)
        (`|ExecutionSequence` :!label _label_6
          (:`then_0`
            (goto _label_3 :!via `Stop`))
          (:`then_1`
            (goto _label_4 :!via `Stop`))
          (:`then_2`
            (goto _label_5))
          (:`then_3`
            (`/Game/Characters/Player/BPs/BP_PlayerCharacter.Request: To Jump End` (`/Game/Characters/Player/FunctionLib/BP_PlayerFunctionLibrary.Get Player Character`))
            (`self.DisableInput` (`GameplayStatics.GetPlayerController` 0))
            (`/Game/Characters/Player/FunctionLib/BP_PlayerFunctionLibrary.UpdateFOV` 85.0 1.0)))))))

(event `InputAxis|Crouch`
  (params (AxisValue :type "Float (single-precision)"))
  (bind _player_character (`/Game/Characters/Player/FunctionLib/BP_PlayerFunctionLibrary.Get Player Character`))
  (if (> AxisValue 0.0)
    (set `self.JumpingDropping` true)
    (set `/Game/Characters/Player/BPs/BP_PlayerCharacter.varJumpDistance` (`self.CalcJumpDistance`) _player_character)
    (set `/Game/Characters/Player/BPs/BP_PlayerCharacter.varJumpHeight` 0.0 _player_character)
    (goto _label_6)))

(fn `CalculateJumpDistance`
  (params (ZipeLineTime :type "Float (double-precision)")))

(fn `ClosestSplineLocation`
  (returns (ClosestSpline :type Integer))
  (locals (TempClosestSpline :type Integer) (PreviousDistance :type "Float (double-precision)") (CurrentDistance :type "Float (double-precision)"))
  (bind _splinepoints (`self.SplinePoints`))
  (for (_ _array_index) _splinepoints
    (bind _returnvalue (`KismetMathLibrary.VSize` (- (`SplineComponent.GetLocationAtSplinePoint` (`self.ZipLine`) _array_index "World") (`self.K2_GetActorLocation` (`/Game/Characters/Player/FunctionLib/BP_PlayerFunctionLibrary.Get Player Character`)))))
    (set `local.CurrentDistance` _returnvalue)
    (if (== _array_index 0)
      (set `local.TempClosestSpline` 0)
      (set `local.PreviousDistance` _returnvalue)
      (elif (< (`local.CurrentDistance`) (`local.PreviousDistance`))
        (set `local.TempClosestSpline` _array_index)
        (set `local.PreviousDistance` (`local.CurrentDistance`)))))
  (`KismetSystemLibrary.PrintString` (`KismetStringLibrary.Conv_IntToString` (`KismetArrayLibrary.Array_Length` _splinepoints)))
  (return (`local.TempClosestSpline`)))

(fn `GetSplinePoints`
  (bind _returnvalue (`SplineComponent.GetNumberOfSplinePoints` (`self.ZipLine`)))
  (for _index (range (+ (- _returnvalue 2) 1))
    (`KismetSystemLibrary.PrintString` (`KismetStringLibrary.Conv_IntToString` _returnvalue))
    (`KismetArrayLibrary.Array_Add` (`self.SplinePoints`) _index)
    (return)))

(fn `UserConstructionScript`
  (bind _bad (`self.Bad`))
  (bind _enddebug (`self.EndDebug`))
  (bind _zipline (`self.ZipLine`))
  (bind _bad_2 (`self.Bad`))
  (bind (_returnvalue_x _returnvalue_y _returnvalue_z) (`KismetMathLibrary.BreakVector` (`SplineComponent.GetLocationAtSplinePoint` (`self.ZipLine`) 0 "Local")))
  (bind (_relativelocation_x _relativelocation_y _relativelocation_z) (`KismetMathLibrary.BreakVector` (`SceneComponent.RelativeLocation` (`self.Bad`))))
  ;[1 0 0.0652] Zipline
  (`|ExecutionSequence`
    (:`then_0`
      (for _index (range (+ (- (`SplineComponent.GetNumberOfSplinePoints` _zipline) 2) 1))
        (bind _returnvalue (+ _index 1))
        (bind _location (`SplineComponent.GetLocationAndTangentAtSplinePoint` _zipline _returnvalue "Local"))
        (`SceneComponent.K2_SetRelativeLocation` (`self.Cable`) _location false false)
        (`|ExecutionSequence`
          (:`then_0`
            (set `self.varEndLocation` (`SplineComponent.GetLocationAndTangentAtSplinePoint` _zipline _returnvalue "Local"))
            (`SceneComponent.K2_SetRelativeLocation` _enddebug (+ _location (* (`SceneComponent.GetRightVector` _enddebug) 90.0)) false false)
            (`SceneComponent.K2_SetRelativeLocation` _bad (+ _location (* (`SceneComponent.GetUpVector` _bad) 40.0)) false false)
            (if (>= _returnvalue_z _relativelocation_z)
              (`SceneComponent.SetVisibility` _bad_2 false false)
              (else
                (`SceneComponent.SetVisibility` _bad_2 true false)
                (set `self.varBad` true))))
          (:`then_1`
            (bind (_returnvalue_roll _returnvalue_pitch _returnvalue_yaw) (`KismetMathLibrary.BreakRotator` (`KismetMathLibrary.FindLookAtRotation` (`SplineComponent.GetLocationAndTangentAtSplinePoint` _zipline _index "Local") _location)))
            (`SceneComponent.K2_SetRelativeRotation` (`self.SM_ZipLine`) (`KismetMathLibrary.MakeRotator` 0.0 0.0 _returnvalue_yaw) false false)
            (`SceneComponent.K2_SetRelativeRotation` (`self.Interact`) (`KismetMathLibrary.MakeRotator` 0.0 0.0 _returnvalue_yaw) false false)
            (`SceneComponent.K2_SetRelativeRotation` (`self.SM_ZipLine1`) (`KismetMathLibrary.MakeRotator` 0.0 0.0 _returnvalue_yaw) false false))
          (:`then_2`
            (`SceneComponent.K2_SetRelativeLocation` (`self.SM_ZipLine1`) _location false false)))))
    (:`then_1`
      (if (> (`SplineComponent.GetNumberOfSplinePoints` (`self.ZipLine`)) 2)
        (`SceneComponent.SetVisibility` (`self.Bad`) true false)
        (set `self.varBad` true)))))