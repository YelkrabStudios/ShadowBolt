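; Dynamic parkour probe that detects climbable ledges for the player character while standing or sprinting, running entirely in the construction script.
; Line traces reshape a spline's points to the surrounding geometry.
; Height and distance tests on key points, plus clearance traces, set the player's climb flag, Climbing or Standing state, climb start/end locations and camera shake.
; A similar vault check exists but is disconnected and never runs.
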(fn `UserConstructionScript`
  (locals (Point5Z :type "Float (double-precision)" :default 0.0) (Point0Z :type "Float (double-precision)" :default 0.0) (ZDifference :type "Float (double-precision)" :default 0.0) (DebugTypeClimb :type "EDrawDebugTrace Enum" :default "None") (DebugTypeVault :type "EDrawDebugTrace Enum" :default "Persistent"))
  (bind _player_character (`/Game/Characters/Player/FunctionLib/BP_PlayerFunctionLibrary.Get Player Character`))
  (bind _player_character_2 (`/Game/Characters/Player/FunctionLib/BP_PlayerFunctionLibrary.Get Player Character`))
  (bind _capsulecomponent (`/Game/Characters/Player/FunctionLib/BP_PlayerFunctionLibrary.GetCapsuleComp`))
  (bind _player_character_3 (`/Game/Characters/Player/FunctionLib/BP_PlayerFunctionLibrary.Get Player Character`))
  (bind _spline (`self.Spline`))
  (bind _spline_2 (`self.Spline`))
  (bind _spline_3 (`self.Spline`))
  (bind _spline_4 (`self.Spline`))
  (bind _spline_5 (`self.Spline`))
  (bind _spline_6 (`self.Spline`))
  (bind _spline_7 (`self.Spline`))
  (bind _spline_8 (`self.Spline`))
  (bind _spline_9 (`self.Spline`))
  (bind _spline_10 (`self.Spline`))
  (bind _spline_11 (`self.Spline`))
  (bind _spline_12 (`self.Spline`))
  (bind _spline_13 (`self.Spline`))
  (bind _spline_14 (`self.Spline`))
  (bind _spline_15 (`self.Spline`))
  (bind _spline_16 (`self.Spline`))
  (bind _spline_17 (`self.Spline`))
  (bind (_returnvalue_x _returnvalue_y _returnvalue_z) (`KismetMathLibrary.BreakVector` (`SplineComponent.GetLocationAtSplinePoint` _spline_17 0 "World")))
  (bind _returnvalue (`SplineComponent.GetLocationAtSplinePoint` _spline_4 5 "World"))
  (bind _returnvalue_2 (`SceneComponent.K2_GetComponentLocation` _capsulecomponent))
  (bind (_returnvalue_x_2 _returnvalue_y_2 _returnvalue_z_2) (`KismetMathLibrary.BreakVector` (`SplineComponent.GetLocationAtSplinePoint` (`self.Spline`) 5 "World")))
  (bind _returnvalue_3 (`SplineComponent.GetLocationAtSplinePoint` _spline_8 5 "World"))
  (bind _returnvalue_4 (`SplineComponent.GetLocationAtSplinePoint` _spline_9 5 "World"))
  (bind _returnvalue_5 (`SplineComponent.GetLocationAtSplinePoint` _spline_10 5 "World"))
  (bind (_returnvalue_x_3 _returnvalue_y_3 _returnvalue_z_3) (`KismetMathLibrary.BreakVector` (`SplineComponent.GetLocationAtSplinePoint` _spline_17 5 "World")))
  (bind _returnvalue_6 (`SplineComponent.GetLocationAtSplinePoint` _spline_2 5 "World"))
  (bind _returnvalue_7 (`KismetMathLibrary.Vector_Distance` (`SplineComponent.GetLocationAtSplinePoint` _spline_6 0 "World") (`SplineComponent.GetLocationAtSplinePoint` _spline_6 5 "World")))
  (bind _returnvalue_8 (+ (`SplineComponent.GetLocationAtSplinePoint` _spline_3 5 "World") (* (`SceneComponent.GetRightVector` _spline_3) -50.0)))
  (bind _returnvalue_9 (+ (`SplineComponent.GetLocationAtSplinePoint` _spline_5 5 "World") (* (`SceneComponent.GetUpVector` _spline_5) 190.0)))
  (bind _returnvalue_10 (+ (`SplineComponent.GetLocationAtSplinePoint` _spline_11 5 "World") (* (`SceneComponent.GetRightVector` _spline_11) 50.0)))
  (bind _returnvalue_11 (+ (`SplineComponent.GetLocationAtSplinePoint` _spline_12 5 "World") (* (`SceneComponent.GetRightVector` _spline_12) -50.0) (* (`SceneComponent.GetForwardVector` _spline_12) 30.0)))
  (bind _returnvalue_12 (+ (`SplineComponent.GetLocationAtSplinePoint` _spline_13 5 "World") (* (`SceneComponent.GetRightVector` _spline_13) 50.0) (* (`SceneComponent.GetForwardVector` _spline_13) 30.0)))
  ;[1 0.03125 0.8087] Request
  (switch `/Game/Characters/Player/Enums/Enum_Player_MovementStates` (`/Game/Characters/Player/FunctionLib/BP_PlayerFunctionLibrary.GetMovementState`)
    (:`NewEnumerator4`
      _)
    (:`NewEnumerator1`
      _))
  (`|ExecutionSequence`
    (:`then_0`
      ;[1 0.03125 0.8087] Point Detector Logic
      (for _index (range (+ (- (`SplineComponent.GetNumberOfSplinePoints` _spline_16) 2) 1))
        (bind _returnvalue_13 (+ _index 1))
        (`KismetArrayLibrary.Array_Add` (`self.SplinePoints`) _returnvalue_13)
        (set `self.Points` _returnvalue_13)
        (`KismetArrayLibrary.Array_Add` (`self.Locations`) (`SplineComponent.GetLocationAtSplinePoint` _spline_16 _returnvalue_13 "World"))
        (for _array_element (`self.Locations`)
          (`|ExecutionSequence`
            (:`then_0`
              (bind (_outhit _returnvalue_14) (`KismetSystemLibrary.LineTraceSingle` :`Start` _array_element :`End` (+ (* (`SceneComponent.GetForwardVector` (`self.Spline`)) 50.0) _array_element) :`TraceChannel` "TraceTypeQuery1" :`DrawTime` 2.0))
              (if _returnvalue_14
                (for _index_2 (range _returnvalue_13 (+ (`SplineComponent.GetNumberOfSplinePoints` _spline_15) 1))
                  (`SplineComponent.SetLocationAtSplinePoint` _spline_15 _index_2 (`KismetMathLibrary.MakeVector` (.x (`.Location` (`GameplayStatics.BreakHitResult` _outhit))) (.y (`.Location` (`GameplayStatics.BreakHitResult` _outhit))) (+ (.z (`.Location` (`GameplayStatics.BreakHitResult` _outhit))) 70.0)) "World" true))
                (else
                  (set `/Game/Characters/Player/BPs/BP_PlayerCharacter.varCanClimb` false (`/Game/Characters/Player/FunctionLib/BP_PlayerFunctionLibrary.Get Player Character`))
                  (for _array_element_2 (`self.Locations`)
                    (`|ExecutionSequence`
                      (:`then_0`
                        (for _index_3 (range _returnvalue_13 (+ (`SplineComponent.GetNumberOfSplinePoints` (`self.Spline`)) 1))
                          (`SplineComponent.SetLocationAtSplinePoint` _spline_14 _index_3 (+ _array_element_2 (* (`SceneComponent.GetForwardVector` _spline_14) 10.0)) "World" true))))))))
            (:`then_1`
              (bind (_outhit_2 _returnvalue_15) (`KismetSystemLibrary.LineTraceSingle` :`Start` _array_element :`End` (+ _array_element (* (`SceneComponent.GetUpVector` (`self.Spline`)) -400.0)) :`TraceChannel` "TraceTypeQuery1" :`DrawTime` 2.0))
              (if _returnvalue_15
                (`SplineComponent.SetLocationAtSplinePoint` _spline _returnvalue_13 (+ (`.Location` (`GameplayStatics.BreakHitResult` _outhit_2)) (* (`SceneComponent.GetUpVector` _spline) (`self.Section5UpLength`))) "World" true)
                (else
                  (set `/Game/Characters/Player/BPs/BP_PlayerCharacter.varCanClimb` false (`/Game/Characters/Player/FunctionLib/BP_PlayerFunctionLibrary.Get Player Character`)))))))))
    (:`then_1`
      (if (== (`/Game/Characters/Player/FunctionLib/BP_PlayerFunctionLibrary.ActiveClimbPoint`) 1)
        (`|ExecutionSequence`
          (:`then_1`
            ;[1 0 0.8672] Detect Can Climb
            (set `local.Point5Z` _returnvalue_z_3)
            (set `local.Point0Z` _returnvalue_z)
            (if (< _returnvalue_z_3 _returnvalue_z)
              (set `self.Point_5_IsUp?` true)
              (set `/Game/Characters/Player/BPs/BP_PlayerCharacter.varCanVault` false _player_character_2)
              (if (and (and (> _returnvalue_7 2.0) (< _returnvalue_7 175.0)) (< (`KismetMathLibrary.Vector_Distance` (`SplineComponent.GetLocationAtSplinePoint` _spline_7 4 "World") (`SplineComponent.GetLocationAtSplinePoint` _spline_7 5 "World")) 40.0))
                ;[0.8984 0 1] Climb Logic
                (`|ExecutionSequence`
                  (:`then_0`
                    (bind (_outhit_3 _returnvalue_16) (`KismetSystemLibrary.LineTraceSingle` :`Start` _returnvalue_2 :`End` (+ _returnvalue_2 (* (`SceneComponent.GetUpVector` _capsulecomponent) _returnvalue_z_2)) :`TraceChannel` "TraceTypeQuery1" :`DrawDebugType` (`local.DebugTypeClimb`) :`TraceColor` (struct :`G` 0.833799 :`B` 1.0 :`A` 1.0) :`DrawTime` 0.0))
                    (if (not _returnvalue_16)
                      (`|ExecutionSequence`
                        (:`then_0`
                          (bind (_outhit_4 _returnvalue_17) (`KismetSystemLibrary.LineTraceSingle` :`Start` _returnvalue :`End` (+ _returnvalue (* (`SceneComponent.GetForwardVector` _spline_4) 30.0)) :`TraceChannel` "TraceTypeQuery1" :`bTraceComplex` true :`DrawDebugType` (`local.DebugTypeClimb`) :`TraceColor` (struct :`R` 1.0 :`G` 0.014541 :`A` 1.0) :`DrawTime` 0.0))
                          (if _returnvalue_17
                            (set `/Game/Characters/Player/BPs/BP_PlayerCharacter.varCanClimb` false (`/Game/Characters/Player/FunctionLib/BP_PlayerFunctionLibrary.Get Player Character`) :!label _label)))
                        (:`then_1`
                          (bind (_outhit_5 _returnvalue_18) (`KismetSystemLibrary.LineTraceSingle` :`Start` _returnvalue_5 :`End` (+ (* (`SceneComponent.GetUpVector` _spline_10) 190.0) _returnvalue_5) :`TraceChannel` "TraceTypeQuery1" :`DrawDebugType` (`local.DebugTypeClimb`) :`DrawTime` 0.0))
                          (if _returnvalue_18
                            (goto _label)
                            (else
                              (bind (_outhit_6 _returnvalue_19) (`KismetSystemLibrary.LineTraceSingle` :`Start` _returnvalue_9 :`End` (+ _returnvalue_9 (* (`SceneComponent.GetForwardVector` _spline_5) 30.0)) :`TraceChannel` "TraceTypeQuery1" :`DrawDebugType` (`local.DebugTypeClimb`) :`DrawTime` 0.0))
                              (if _returnvalue_19
                                (set `/Game/Characters/Player/BPs/BP_PlayerCharacter.varCanClimb` false (`/Game/Characters/Player/FunctionLib/BP_PlayerFunctionLibrary.Get Player Character`))
                                (else
                                  (`|ExecutionSequence`
                                    (:`then_0`
                                      (bind (_outhit_7 _returnvalue_20) (`KismetSystemLibrary.LineTraceSingle` :`Start` _returnvalue_4 :`End` (+ (* (`SceneComponent.GetRightVector` _spline_9) 50.0) _returnvalue_4) :`TraceChannel` "TraceTypeQuery1" :`DrawDebugType` (`local.DebugTypeClimb`) :`DrawTime` 0.0))
                                      (if _returnvalue_20
                                        (set `/Game/Characters/Player/BPs/BP_PlayerCharacter.varCanClimb` false (`/Game/Characters/Player/FunctionLib/BP_PlayerFunctionLibrary.Get Player Character`))
                                        (else
                                          (bind (_outhit_8 _returnvalue_21) (`KismetSystemLibrary.LineTraceSingle` :`Start` _returnvalue_10 :`End` (+ _returnvalue_10 (* (`SceneComponent.GetForwardVector` _spline_11) 30.0)) :`TraceChannel` "TraceTypeQuery1" :`DrawDebugType` (`local.DebugTypeClimb`) :`DrawTime` 0.0))
                                          (if _returnvalue_21
                                            (set `/Game/Characters/Player/BPs/BP_PlayerCharacter.varCanClimb` false (`/Game/Characters/Player/FunctionLib/BP_PlayerFunctionLibrary.Get Player Character`) :!label _label_2)
                                            (else
                                              (bind (_outhit_9 _returnvalue_22) (`KismetSystemLibrary.LineTraceSingle` :`Start` _returnvalue_12 :`End` (+ (* (`SceneComponent.GetUpVector` _spline_13) 190.0) _returnvalue_12) :`TraceChannel` "TraceTypeQuery1" :`DrawDebugType` (`local.DebugTypeClimb`) :`DrawTime` 0.0))
                                              (if _returnvalue_22
                                                (goto _label_2)))))))
                                    (:`then_1`
                                      (bind (_outhit_10 _returnvalue_23) (`KismetSystemLibrary.LineTraceSingle` :`Start` _returnvalue_3 :`End` (+ _returnvalue_3 (* (`SceneComponent.GetRightVector` _spline_8) -50.0)) :`TraceChannel` "TraceTypeQuery1" :`DrawDebugType` (`local.DebugTypeClimb`) :`DrawTime` 0.0))
                                      (if _returnvalue_23
                                        (set `/Game/Characters/Player/BPs/BP_PlayerCharacter.varCanClimb` false (`/Game/Characters/Player/FunctionLib/BP_PlayerFunctionLibrary.Get Player Character`))
                                        (else
                                          (bind (_outhit_11 _returnvalue_24) (`KismetSystemLibrary.LineTraceSingle` :`Start` _returnvalue_8 :`End` (+ _returnvalue_8 (* (`SceneComponent.GetForwardVector` _spline_3) 30.0)) :`TraceChannel` "TraceTypeQuery1" :`DrawDebugType` (`local.DebugTypeClimb`) :`DrawTime` 0.0))
                                          (if _returnvalue_24
                                            (goto _label_2)
                                            (else
                                              (bind (_outhit_12 _returnvalue_25) (`KismetSystemLibrary.LineTraceSingle` :`Start` _returnvalue_11 :`End` (+ (* (`SceneComponent.GetUpVector` _spline_12) 190.0) _returnvalue_11) :`TraceChannel` "TraceTypeQuery1" :`DrawDebugType` (`local.DebugTypeClimb`) :`DrawTime` 0.0))
                                              (if _returnvalue_25
                                                (goto _label_2))))))))))))))))
                  (:`then_1`
                    (if (or _returnvalue_16 _returnvalue_17 _returnvalue_18 _returnvalue_19 _returnvalue_23 _returnvalue_20 _returnvalue_24 _returnvalue_21 _returnvalue_25 _returnvalue_22)
                      (set `/Game/Characters/Player/BPs/BP_PlayerCharacter.varMovementState` "NewEnumerator1" _player_character_3)
                      (else
                        (bind _output_get (set `/Game/Characters/Player/BPs/BP_PlayerCharacter.varMovementState` "NewEnumerator9" _player_character_3))
                        (if (`|EnumEquality` _output_get "NewEnumerator9")
                          (`|ExecutionSequence`
                            (:`then_0`
                              (set `/Game/Characters/Player/BPs/BP_PlayerCharacter.varClimbEndLocation` (`SplineComponent.GetLocationAtSplinePoint` (`self.Spline`) 5 "World") (`/Game/Characters/Player/FunctionLib/BP_PlayerFunctionLibrary.Get Player Character`)))
                            (:`then_1`
                              (bind (_outhit_13 _returnvalue_26) (`KismetSystemLibrary.LineTraceSingle` :`Start` (+ (* (`SceneComponent.GetForwardVector` _spline_2) -100.0) _returnvalue_6) :`End` (+ _returnvalue_6 (* (`SceneComponent.GetUpVector` _spline_2) -3.0)) :`TraceChannel` "TraceTypeQuery1" :`DrawDebugType` "Persistent" :`TraceColor` (struct :`R` 1.0 :`B` 0.067656 :`A` 1.0)))
                              (if _returnvalue_26
                                (set `/Game/Characters/Player/BPs/BP_PlayerCharacter.varClimbStartLocation` (`.Location` (`GameplayStatics.BreakHitResult` _outhit_13)) _player_character)
                                (`/Game/Characters/Player/FunctionLib/BP_PlayerFunctionLibrary.PlayCameraShake` "/Game/Characters/Player/Misc/CameraShake/Movement/Jump/BP_JumpeEndCameraShake.BP_JumpeEndCameraShake_C" 4.0)
                                (else
                                  (set `/Game/Characters/Player/BPs/BP_PlayerCharacter.varCanClimb` false _player_character))))))))))
                (else
                  (set `/Game/Characters/Player/BPs/BP_PlayerCharacter.varCanClimb` false _player_character_2 :!label _label_3)))
              (else
                (set `self.Point_5_IsUp?` false)
                (goto _label_3)))))))))